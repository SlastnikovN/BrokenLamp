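; BP_BasePlayer is the base player pawn, providing movement, interaction with world objects and on-screen text reactions.
; InteractableArea overlaps maintain a list of BP_InteractableActor, and press, hold and tap interactions message its first entry with the player as argument.
; Move converts a direction into world-space movement input with X negated.
; ShowReaction sets text on a BPW_CharacterReactionWidget component, shows it, then hides it after a delay.
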(event `self.InteractableArea.OnComponentBeginOverlap`
  (params (OverlappedComponent :type "PrimitiveComponent Object Reference") (OtherActor :type "Actor Object Reference") (OtherComp :type "PrimitiveComponent Object Reference") (OtherBodyIndex :type Integer) (bFromSweep :type Boolean) (SweepResult :type "HitResult Structure (by ref)"))
  (bind _asbp_interactable_actor (cast `/Game/Blueprints/Interaction/BP_InteractableActor` OtherActor))
  (`KismetArrayLibrary.Array_Add` (`self.FocusedInteractableActor`) _asbp_interactable_actor))

(event `self.InteractableArea.OnComponentEndOverlap`
  (params (OverlappedComponent :type "PrimitiveComponent Object Reference") (OtherActor :type "Actor Object Reference") (OtherComp :type "PrimitiveComponent Object Reference") (OtherBodyIndex :type Integer))
  (bind _asbp_interactable_actor (cast `/Game/Blueprints/Interaction/BP_InteractableActor` OtherActor))
  (`KismetArrayLibrary.Array_RemoveItem` (`self.FocusedInteractableActor`) _asbp_interactable_actor))

(event `ShowReaction`
  (params (ReactionText :type Text))
  (bind _asbpw_character_reaction_widget (cast `/Game/Blueprints/Widgets/Characters/BPW_CharacterReactionWidget` (`WidgetComponent.GetWidget` (`self.Widget`))))
  (`/Game/Blueprints/Widgets/Characters/BPW_CharacterReactionWidget.SetReactionText` _asbpw_character_reaction_widget ReactionText)
  (`SceneComponent.SetVisibility` (`self.Widget`) true false)
  (`KismetSystemLibrary.Delay` (`self.ShowReactionDuration`))
  (`SceneComponent.SetVisibility` (`self.Widget`) false false))

(fn `HoldInteract`
  (bind _output (`|GetArrayItem` (`self.FocusedInteractableActor`)))
  (`/Engine/EditorBlueprintResources/StandardMacros.IsValid` _output
    (:`Is Valid`
      (message `/Game/Blueprints/Interaction/BPI_Interactable.HoldInteract` _output self)
      (return))))

(fn `Move`
  (params (Direction :type "Vector2D Structure"))
  (`self.AddMovementInput` (`KismetMathLibrary.MakeVector` (* Direction_X -1.0) Direction_Y))
  (return))

(fn `PressInteract`
  (bind _output (`|GetArrayItem` (`self.FocusedInteractableActor`)))
  (`/Engine/EditorBlueprintResources/StandardMacros.IsValid` _output
    (:`Is Valid`
      (message `/Game/Blueprints/Interaction/BPI_Interactable.PressInteract` _output self)
      (return))))

(fn `TapInteract`
  (bind _output (`|GetArrayItem` (`self.FocusedInteractableActor`)))
  (`/Engine/EditorBlueprintResources/StandardMacros.IsValid` _output
    (:`Is Valid`
      (message `/Game/Blueprints/Interaction/BPI_Interactable.TapInteract` _output self)
      (return))))

(fn `UserConstructionScript`)