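; Player controller that drives both Anna and Leon from one shared Enhanced Input mapping context.
; On BeginPlay it finds both characters in the level, using a FlipFlop as a join to record their starting locations once both are found.
; Per-character input actions forward movement and press, tap or hold interaction, while caching move input and last/current locations.
; Escape toggles the menu widget, switching input mode and pausing via zero global time dilation.
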(event `self.ReceiveBeginPlay`
  (bind _returnvalue (`self.K2_GetActorLocation` (`self.Anna`)))
  (bind _returnvalue_2 (`self.K2_GetActorLocation` (`self.Leon`)))
  (`|ExecutionSequence`
    (:`then_0`
      (`EnhancedInputSubsystemInterface.AddMappingContext` (subsystem `EnhancedInputLocalPlayerSubsystem`) "/Game/Blueprints/Core/Input/IMC_TwoPlayersInputContext.IMC_TwoPlayersInputContext" 0 (struct)))
    (:`then_1`
      ; Find Characters on level
      (bind _returnvalue_3 (`GameplayStatics.GetActorOfClass` "/Game/Blueprints/Core/BP_Anna.BP_Anna_C"))
      (`/Engine/EditorBlueprintResources/StandardMacros.IsValid` _returnvalue_3
        (:`Is Valid`
          (set `self.Anna` _returnvalue_3)
          (`/Engine/EditorBlueprintResources/StandardMacros.FlipFlop` :!label _label
            (:`B`
              (`KismetSystemLibrary.PrintString` "All characters successfuly finded!!" false)
              ; Save Characters locations
              (set `self.AnnaCurrentLocation` _returnvalue)
              (set `self.AnnaLastLocation` _returnvalue)
              (set `self.LeonCurrentLocation` _returnvalue_2)
              (set `self.LeonLastLocation` _returnvalue_2))))))
    (:`then_2`
      (bind _returnvalue_4 (`GameplayStatics.GetActorOfClass` "/Game/Blueprints/Core/BP_Leon.BP_Leon_C"))
      (`/Engine/EditorBlueprintResources/StandardMacros.IsValid` _returnvalue_4
        (:`Is Valid`
          (set `self.Leon` _returnvalue_4)
          (goto _label))))))

(event `OnMenuSelflyClosed`
  (`Widget.RemoveFromParent` (`self.MenuWidget`) :!label _label_2)
  (set `self.MenuWidget` null)
  (set `self.bShowMouseCursor` false)
  (`WidgetBlueprintLibrary.SetInputMode_GameOnly` self)
  (`GameplayStatics.SetGlobalTimeDilation` 1.0))

(event `Key|Escape`
  (params (Key :type "Key Structure"))
  (:`Pressed`
    (`/Engine/EditorBlueprintResources/StandardMacros.IsValid` (`self.MenuWidget`)
      (:`Is Valid`
        (goto _label_2))
      (:`Is Not Valid`
        (bind _returnvalue (`|CreateWidget` "/Game/Blueprints/Widgets/Menu/BPW_Menu.BPW_Menu_C"))
        (bind _output_get (set `self.MenuWidget` _returnvalue))
        (add `/Game/Blueprints/Widgets/Menu/BPW_Menu.ContinueButtonPressed` _output_get (`|CreateDelegate` :!event `OnMenuSelflyClosed`))
        (`UserWidget.AddToViewport` _output_get 0)
        (set `self.bShowMouseCursor` true)
        (`WidgetBlueprintLibrary.SetInputMode_GameAndUIEx` self (`self.MenuWidget`))
        (`GameplayStatics.SetGlobalTimeDilation` 0.0)))))

(event `EnhancedInput|/Game/Blueprints/Core/Input/Actions/IA_LeonMove`
  (params (ActionValue :type "Vector2D Structure") (ElapsedSeconds :type "Float (double-precision)") (TriggeredSeconds :type "Float (double-precision)") (InputAction :type "InputAction Object Reference" :default "/Game/Blueprints/Core/Input/Actions/IA_LeonMove.IA_LeonMove"))
  ; Movement
  (:`Triggered`
    (set `self.LeonLastLocation` (`SceneComponent.K2_GetComponentLocation` (`Actor.RootComponent` (`self.Leon`))))
    (`/Game/Blueprints/Core/BP_BasePlayer.Move` (`self.Leon`) ActionValue)
    (set `self.LeonMovement` ActionValue)
    (set `self.LeonCurrentLocation` (`SceneComponent.K2_GetComponentLocation` (`Actor.RootComponent` (`self.Leon`)))))
  (:`Completed`
    (set `self.LeonMovement` (0.0 0.0))))

(event `EnhancedInput|/Game/Blueprints/Core/Input/Actions/IA_AnnaInteraction`
  (params (ActionValue :type Boolean) (ElapsedSeconds :type "Float (double-precision)") (TriggeredSeconds :type "Float (double-precision)") (InputAction :type "InputAction Object Reference" :default "/Game/Blueprints/Core/Input/Actions/IA_AnnaInteraction.IA_AnnaInteraction"))
  (bind _anna (`self.Anna`))
  (bind _anna_2 (`self.Anna`))
  ; Interaction
  (:`Started`
    (`/Engine/EditorBlueprintResources/StandardMacros.IsValid` _anna_2
      (:`Is Valid`
        (`/Game/Blueprints/Core/BP_BasePlayer.PressInteract` _anna_2)
        (`/Game/Blueprints/Core/BP_BasePlayer.TapInteract` _anna_2))))
  (:`Ongoing`
    (`/Engine/EditorBlueprintResources/StandardMacros.IsValid` _anna
      (:`Is Valid`
        (`/Game/Blueprints/Core/BP_BasePlayer.HoldInteract` _anna)))))

(event `EnhancedInput|/Game/Blueprints/Core/Input/Actions/IA_AnnaMove`
  (params (ActionValue :type "Vector2D Structure") (ElapsedSeconds :type "Float (double-precision)") (TriggeredSeconds :type "Float (double-precision)") (InputAction :type "InputAction Object Reference" :default "/Game/Blueprints/Core/Input/Actions/IA_AnnaMove.IA_AnnaMove"))
  ; Movement
  (:`Triggered`
    (set `self.AnnaLastLocation` (`self.K2_GetActorLocation` (`self.Anna`)))
    (`/Game/Blueprints/Core/BP_BasePlayer.Move` (`self.Anna`) ActionValue)
    (set `self.AnnaMovement` ActionValue)
    (set `self.AnnaCurrentLocation` (`self.K2_GetActorLocation` (`self.Anna`))))
  (:`Completed`
    (set `self.AnnaMovement` (0.0 0.0))))

(event `EnhancedInput|/Game/Blueprints/Core/Input/Actions/IA_LeonInteraction`
  (params (ActionValue :type Boolean) (ElapsedSeconds :type "Float (double-precision)") (TriggeredSeconds :type "Float (double-precision)") (InputAction :type "InputAction Object Reference" :default "/Game/Blueprints/Core/Input/Actions/IA_LeonInteraction.IA_LeonInteraction"))
  (bind _leon (`self.Leon`))
  (bind _leon_2 (`self.Leon`))
  ; Interaction
  (:`Started`
    (`/Engine/EditorBlueprintResources/StandardMacros.IsValid` _leon
      (:`Is Valid`
        (`/Game/Blueprints/Core/BP_BasePlayer.PressInteract` _leon)
        (`/Game/Blueprints/Core/BP_BasePlayer.TapInteract` _leon))))
  (:`Ongoing`
    (`/Engine/EditorBlueprintResources/StandardMacros.IsValid` _leon_2
      (:`Is Valid`
        (`/Game/Blueprints/Core/BP_BasePlayer.HoldInteract` _leon_2)))))

(fn `UserConstructionScript`)