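; An interactable actor Blueprint that plays a Level Sequence when its interaction completes.
; It overrides CompleteInteraction, runs the parent logic, then, if a LevelSequence is assigned, creates a sequence player at runtime and plays it.
; Playback settings disable movement input during the sequence.
; The event graph holds only disabled default events, so all added behavior lives in that override.
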(fn `CompleteInteraction`
  (bind _levelsequence (`self.LevelSequence`))
  (`parent.CompleteInteraction`)
  (`/Engine/EditorBlueprintResources/StandardMacros.IsValid` _levelsequence
    (:`Is Valid`
      (bind _outactor (`LevelSequencePlayer.CreateLevelSequencePlayer` _levelsequence (make `MovieSceneSequencePlaybackSettings` false (struct) (struct :`bAllowRounding` true) 1.0 0.0 false true)))
      (`MovieSceneSequencePlayer.Play` (`LevelSequenceActor.SequencePlayer` _outactor)))))

(fn `UserConstructionScript`
  (`parent.UserConstructionScript`))