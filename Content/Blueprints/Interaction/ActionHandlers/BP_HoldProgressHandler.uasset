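; Interaction action handler that tracks hold progress toward a destination value.
; AddProgress accumulates input into HoldProgress, fires an update, then latches Completed and fires completion when progress is within a small tolerance of the destination.
; Completion uses a near-equality check, so an overshoot beyond the tolerance does not complete it.
; Once completed, further calls only fire the update without changing progress.
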(fn `AddProgress`
  (params (InputValue :type "Float (double-precision)"))
  (if (not (`self.bCompleted`))
    (set `self.HoldProgress` (+ (`self.HoldProgress`) InputValue))
    (`self.HoldProgressUpdated`)
    (if (`KismetMathLibrary.NearlyEqual_FloatFloat` (`self.HoldProgress`) (`self.HoldDestinationProgress`) 0.1)
      (set `self.bCompleted` true)
      (`self.HoldProgressCompleted`)
      (return))
    (else
      (`self.HoldProgressUpdated`))))