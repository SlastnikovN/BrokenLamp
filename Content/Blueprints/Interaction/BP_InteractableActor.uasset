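; Interactable world actor that shows an interaction widget when the required character, Anna, Leon or both, is in its area.
; BeginPlay configures the widget from ActorInteractionInfo.
; Each Tick, CheckCanInteract scans InteractableArea overlaps and toggles widget visibility; it blocks once Completed, and its per-character flags are never cleared.
; PressInteract fires CallPressCompleted; hold, tap, process and complete hooks are empty.
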(event `self.ReceiveBeginPlay`
  (bind (_actorinteractioninfo_interactiontype _actorinteractioninfo_interactionsocialtype) (break `/Game/Blueprints/Interaction/S_ObjectInteractionInfo` (`self.ActorInteractionInfo`)))
  (bind _asbpw_interaction_type_widget (cast `/Game/Blueprints/Widgets/Actors/BPW_InteractionTypeWidget` (`WidgetComponent.GetWidget` (`self.Widget`))))
  (`/Game/Blueprints/Widgets/Actors/BPW_InteractionTypeWidget.SetType` _asbpw_interaction_type_widget _actorinteractioninfo_interactiontype _actorinteractioninfo_interactionsocialtype))

(event `self.ReceiveTick`
  (params (DeltaSeconds :type "Float (single-precision)"))
  (`self.CheckCanInteract`)
  (if (`self.bCanInteract`)
    (`SceneComponent.SetVisibility` (`self.Widget`) true false)
    (else
      (`SceneComponent.SetVisibility` (`self.Widget`) false false))))

(event `/Game/Blueprints/Interaction/BPI_Interactable.PressInteract`
  (params (InvistigaterCharacter :type "/Game/Blueprints/Core/BP_BasePlayer Object Reference"))
  (`self.PressCompleted`))

(event `/Game/Blueprints/Interaction/BPI_Interactable.HoldInteract`
  (params (InvistigaterCharacter :type "/Game/Blueprints/Core/BP_BasePlayer Object Reference")))

(event `/Game/Blueprints/Interaction/BPI_Interactable.TapInteract`
  (params (InvistigaterCharacter :type "/Game/Blueprints/Core/BP_BasePlayer Object Reference")))

(fn `CheckCanInteract`
  (locals (ContainsLeon :type Boolean) (ContainsAnna :type Boolean))
  (bind (_actorinteractioninfo_interactiontype _actorinteractioninfo_interactionsocialtype) (break `/Game/Blueprints/Interaction/S_ObjectInteractionInfo` (`self.ActorInteractionInfo`)))
  (if (`self.bCompleted`)
    (set `self.bCanInteract` false)
    (else
      (for _array_element (`PrimitiveComponent.GetOverlappingActors` (`self.InteractableArea`) "/Game/Blueprints/Core/BP_BasePlayer.BP_BasePlayer_C")
        (`|ExecutionSequence`
          (:`then_0`
            (bind _returnvalue (`GameplayStatics.ObjectIsA` _array_element "/Game/Blueprints/Core/BP_Leon.BP_Leon_C"))
            (if _returnvalue
              (set `local.ContainsLeon` _returnvalue)))
          (:`then_1`
            (bind _returnvalue_2 (`GameplayStatics.ObjectIsA` _array_element "/Game/Blueprints/Core/BP_Anna.BP_Anna_C"))
            (if _returnvalue_2
              (set `local.ContainsAnna` _returnvalue_2)))))
      (switch `/Game/Blueprints/Interaction/E_InteractionSocialType` _actorinteractioninfo_interactionsocialtype
        (:`NewEnumerator0`
          (set `self.bCanInteract` (`local.ContainsAnna`)))
        (:`NewEnumerator1`
          (set `self.bCanInteract` (`local.ContainsLeon`)))
        (:`NewEnumerator2`
          (set `self.bCanInteract` (and (`local.ContainsLeon`) (`local.ContainsAnna`))))))))

(fn `CompleteInteraction`)

(fn `ProccesInteraction`)

(fn `UserConstructionScript`)