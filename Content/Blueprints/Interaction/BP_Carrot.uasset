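; BP_Carrot is an interactable carrot that stays hidden until the snowman game is completed, then can be collected with a press.
; On BeginPlay it hides its mesh, disables the interaction area's collision and binds to SnowmanGame's completion event, which restores visibility and query-only collision.
; A press passing the can-interact check prints a debug message, sets Completed and destroys the actor.
; Hold interaction is left empty.
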(event `self.ReceiveBeginPlay`
  (`parent.ReceiveBeginPlay`)
  (`SceneComponent.SetVisibility` (`self.StaticMesh_0`) false false)
  (`PrimitiveComponent.SetCollisionEnabled` (`self.InteractableArea`) "NoCollision")
  (add `/Game/Blueprints/Games/Snowman/BP_SnowmanGame.SnowmanCompleted` (`self.SnowmanGame`) (delegate `SnowmanCompleted_Event`)))

(event `SnowmanCompleted_Event`
  (`SceneComponent.SetVisibility` (`self.StaticMesh_0`) true false)
  (`PrimitiveComponent.SetCollisionEnabled` (`self.InteractableArea`) "QueryOnly"))

(event `/Game/Blueprints/Interaction/BPI_Interactable.HoldInteract`
  (params (InvistigaterCharacter :type "/Game/Blueprints/Core/BP_BasePlayer Object Reference")))

(event `/Game/Blueprints/Interaction/BPI_Interactable.PressInteract`
  (params (InvistigaterCharacter :type "/Game/Blueprints/Core/BP_BasePlayer Object Reference"))
  (`self.CheckCanInteract`)
  (if (`self.bCanInteract`)
    (`KismetSystemLibrary.PrintString` "Hello")
    (set `self.bCompleted` true)
    (`self.K2_DestroyActor`)))

(fn `UserConstructionScript`
  (`parent.UserConstructionScript`))