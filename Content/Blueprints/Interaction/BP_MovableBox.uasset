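; BP_MovableBox is an interactable box that a character pushes while holding interact.
; HoldInteract line-traces ahead of the character and sweeps the box along the mesh's forward vector, gated on CanInteract and character velocity or controller movement input.
; Its hit-actor check reads from a trace-results loop that never runs.
; Component hits set player-contact and stop flags, which the push ignores.
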(event Custom|OnComponentHit_Event
  (params (HitComponent :type Primitive%20Component%20Object%20Reference) (OtherActor :type Actor%20Object%20Reference) (OtherComp :type Primitive%20Component%20Object%20Reference) (NormalImpulse :type Vector) (Hit :type Hit%20Result%20Structure%20%28by%20ref%29))
  (if (Class|GameplayStatics|ObjectIsA OtherActor "/Game/Blueprints/Core/BP_BasePlayer.BP_BasePlayer_C")
    (Variables|Default|SetbShouldStop false)
    (Variables|Default|SetbHitPlayer true)
    (else
      (Variables|Default|SetbShouldStop true)
      (Variables|Default|SetbHitPlayer false))))

(event EventBeginPlay
  (|CallParentFunction)
  (Collision|AssignOnComponentHit (Variables|Default|GetStaticMesh) (delegate Custom|OnComponentHit_Event)))

(event Collision|EventActorBeginOverlap
  (params (OtherActor :type Actor%20Object%20Reference))
  (|CallParentFunction OtherActor) ; This node is disabled and will not be called.\nDrag off pins to build functionality.
)

(event EventTick
  (params (DeltaSeconds :type Float%20%28single-precision%29))
  (|CallParentFunction DeltaSeconds) ; This node is disabled and will not be called.\nDrag off pins to build functionality.
)

(event EventHoldInteract
  (params (InvistigaterCharacter :type BP%20Base%20Player%20Object%20Reference))
  (bind _returnvalue (Transformation|GetActorLocation InvistigaterCharacter))
  (bind _mesh (Variables|/Script/Engine.Character|GetMesh InvistigaterCharacter))
  (bind _returnvalue_2 (Math|Vector|GetForwardVector _mesh))
  (CallFunction|CheckCanInteract)
  (if (Variables|Default|GetbCanInteract)
    (bind _asbp_two_characters_controller (Utilities|Casting|CastToBP_TwoCharactersController (Game|GetPlayerController 0)))
    (bind _outhits (Collision|MultiLineTraceByChannel _returnvalue (+ _returnvalue (* _returnvalue_2 1e+02)) "TraceTypeQuery1" false (Utilities|Array|MakeArray InvistigaterCharacter) "ForOneFrame" false))
    (if (Math|Boolean|ANDBoolean (Class|GameplayStatics|ObjectIsA (.HitActor (Collision|BreakHitResult (stale _array_element))) "BP_MovableBox_C") (or (not (Utilities|Operators|EqualEqual :A (Variables|/Script/Engine.MovementComponent|GetVelocity (Variables|/Script/Engine.Character|GetCharacterMovement InvistigaterCharacter)))) (not (Class|KismetMathLibrary|IsNearlyZero2D (Variables|/Game/Blueprints/Core/BP_TwoCharactersController.BP_TwoCharactersController_C|GetAnnaMovement _asbp_two_characters_controller) 0.1))) true true)
      (bind _sweephitresult (Transformation|AddActorWorldOffset (* _returnvalue_2 1.0) true))
      (Development|PrintString (Utilities|GetDisplayName (.HitActor (Collision|BreakHitResult _sweephitresult)))))))

(fn ConstructionScript
  (|CallParentFunction))