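; Hold-to-use lever that drives the vertical offset of a linked crane (Cran).
; HoldInteract passes the character to BPHoldInteractionHandler after a CanInteract check, with the hold limit disabled at BeginPlay.
; Each hold update pitches the lever from its initial rotation and calls AddUpOffset on the crane, both scaled by current hold seconds.
; The initial rotation is captured in world space but applied as relative; the saved crane start location is unused.
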(event `self.ReceiveBeginPlay`
  (bind _bp_holdinteractionhandler (`self.BP_HoldInteractionHandler`))
  (bind _cran (`self.Cran`))
  (`parent.ReceiveBeginPlay`)
  (`|ExecutionSequence`
    (:`then_0`
      (`/Engine/EditorBlueprintResources/StandardMacros.IsValid` _bp_holdinteractionhandler
        (:`Is Valid`
          (set `/Game/Blueprints/Interaction/ActionHandlers/BP_HoldInteractionHandler.bLimited` false _bp_holdinteractionhandler)
          (set `self.InitialRotation` (`SceneComponent.K2_GetComponentRotation` (`self.Lever`)))
          (`/Engine/EditorBlueprintResources/StandardMacros.IsValid` _cran
            (:`Is Valid`
              (set `self.CranInitialLocation` (`SceneComponent.K2_GetComponentLocation` (`Actor.RootComponent` _cran))))))))
    (:`then_1`
      (add `/Game/Blueprints/Interaction/ActionHandlers/BP_HoldInteractionHandler.HoldUpdated` (`self.BP_HoldInteractionHandler`) (delegate `HoldUpdated_Event`)))))

(event `HoldUpdated_Event`
  (bind _cran (`self.Cran`))
  (`SceneComponent.K2_SetRelativeRotation` (`self.Lever`) (`KismetMathLibrary.ComposeRotators` (`self.InitialRotation`) (`KismetMathLibrary.MakeRotator` 0.0 (* (`/Game/Blueprints/Interaction/ActionHandlers/BP_HoldInteractionHandler.CurrentHoldSeconds` (`self.BP_HoldInteractionHandler`)) 10.0))) false false)
  (`/Engine/EditorBlueprintResources/StandardMacros.IsValid` _cran
    (:`Is Valid`
      (`/Game/Blueprints/Games/Cran/BP_Cran.AddUpOffset` _cran (+ (0.0 0.0 0.0) (`KismetMathLibrary.MakeVector` 0.0 0.0 (* (`/Game/Blueprints/Interaction/ActionHandlers/BP_HoldInteractionHandler.CurrentHoldSeconds` (`self.BP_HoldInteractionHandler`)) 10.0)))))))

(event `/Game/Blueprints/Interaction/BPI_Interactable.HoldInteract`
  (params (InvistigaterCharacter :type "/Game/Blueprints/Core/BP_BasePlayer Object Reference"))
  (`self.CheckCanInteract`)
  (if (`self.bCanInteract`)
    (`/Game/Blueprints/Interaction/ActionHandlers/BP_HoldInteractionHandler.Hold` (`self.BP_HoldInteractionHandler`) InvistigaterCharacter)))

(fn `UserConstructionScript`
  (`parent.UserConstructionScript`))