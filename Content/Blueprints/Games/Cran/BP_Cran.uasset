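; Crane actor for the Cran game whose 3Crane component moves to vertical and sideways offsets from its starting position.
; AddUpOffset and AddRightOffset replace, rather than accumulate, their offset and fire the UpdateLocation dispatcher, which the actor binds at BeginPlay.
; The handler eases the component over a short time, passing the saved world location plus offsets as a relative target.
; Hit handling and a swept-move alternative are unused.
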(event `self.ReceiveBeginPlay`
  (set `self.InitialLocaiton` (`SceneComponent.K2_GetComponentLocation` (`self.3_Crane`)))
  (`PrimitiveComponent.SetCollisionEnabled` (`self.3_Crane`) "QueryAndPhysics")
  (add `self.UpdateLocation` (delegate `UpdateLocation_Event`)))

(event `UpdateLocation_Event`
  (`KismetSystemLibrary.MoveComponentTo` (`self.3_Crane`) (+ (`self.InitialLocaiton`) (`self.UpOffset`) (`self.RightOffset`)) (struct) false false 0.2)
  (`KismetSystemLibrary.PrintString` (`KismetSystemLibrary.GetDisplayName` null)))

(event `self.3_Crane.OnComponentHit`
  (params (HitComponent :type "PrimitiveComponent Object Reference") (OtherActor :type "Actor Object Reference") (OtherComp :type "PrimitiveComponent Object Reference") (NormalImpulse :type "Vector Structure") (Hit :type "HitResult Structure (by ref)")))

(fn `AddRightOffset`
  (params (RightOffset :type "Vector Structure"))
  (set `self.RightOffset` RightOffset)
  (`self.UpdateLocation`)
  (return))

(fn `AddUpOffset`
  (params (UpOffset :type "Vector Structure"))
  (set `self.UpOffset` UpOffset)
  (`self.UpdateLocation`)
  (return))

(fn `UserConstructionScript`)