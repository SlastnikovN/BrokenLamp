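; Interactable snowball for the snowman minigame, first rolled to grow, then held to place on the snowman.
; Hold input feeds Leon's movement into a progress handler, whose updates scale and shift the ball.
; At max size near a free AnnaPlace, the correct ball snaps in and switches to placement, while a wrong one triggers Anna's reaction.
; Further holding moves it along the game's spline until completion marks it part of the snowman.
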(event `HoldUpdated_Event`
  (bind _snowmangame (`self.SnowmanGame`))
  (`/Engine/EditorBlueprintResources/StandardMacros.IsValid` _snowmangame
    (:`Is Valid`
      (`/Game/Blueprints/Games/Snowman/BP_SnowmanGame.MoveSnowAlongSpline` _snowmangame self))))

(event `HoldCompleted`
  (`KismetSystemLibrary.PrintString` "Hello")
  (set `self.bCompleted` true)
  (set `self.bSnowPartOfSnowMan` true)
  (`self.SnowCompleted`))

(event `HoldProgressCompleted_Event`
  (set `self.bSnowHasMaxShape` true)
  (`self.SnowMaxShapeCompleted`))

(event `self.ReceiveBeginPlay`
  (`parent.ReceiveBeginPlay`)
  (add `/Game/Blueprints/Interaction/ActionHandlers/BP_HoldProgressHandler.HoldProgressUpdated` (`self.BP_HoldProgressHandler`) (delegate `HoldProgressUpdated_Event`))
  (add `/Game/Blueprints/Interaction/ActionHandlers/BP_HoldProgressHandler.HoldProgressCompleted` (`self.BP_HoldProgressHandler`) (delegate `HoldProgressCompleted_Event`))
  (add `/Game/Blueprints/Interaction/ActionHandlers/BP_HoldInteractionHandler.HoldCompleted` (`self.BP_HoldInteractionHandler`) (delegate `HoldCompleted`))
  (add `/Game/Blueprints/Interaction/ActionHandlers/BP_HoldInteractionHandler.HoldUpdated` (`self.BP_HoldInteractionHandler`) (delegate `HoldUpdated_Event`)))

(event `HoldProgressUpdated_Event`
  (bind _result (`/Game/Blueprints/Games/Snowman/BP_SnowmanGame.IsNowRightSnow` (`self.SnowmanGame`) self))
  (bind _returnvalue (`SceneComponent.K2_GetComponentLocation` (`/Game/Blueprints/Games/Snowman/BP_SnowmanGame.AnnaPlace` (`self.SnowmanGame`))))
  (bind _returnvalue_2 (== (`SceneComponent.K2_GetComponentLocation` (`self.StaticMesh`)) _returnvalue :`ErrorTolerance` 10.0))
  (`SceneComponent.SetWorldScale3D` (`self.Scene`) (`KismetMathLibrary.Conv_DoubleToVector` (/ (* (`/Game/Blueprints/Interaction/ActionHandlers/BP_HoldProgressHandler.HoldProgress` (`self.BP_HoldProgressHandler`)) 0.2) 1.0)))
  (`self.SnowUpdated`)
  (bind _asbp_two_characters_controller (cast `/Game/Blueprints/Core/BP_TwoCharactersController` (`GameplayStatics.GetPlayerController` 0)))
  (bind (_leonmovement_x _leonmovement_y) (`KismetMathLibrary.BreakVector2D` (`/Game/Blueprints/Core/BP_TwoCharactersController.LeonMovement` _asbp_two_characters_controller)))
  (`SceneComponent.K2_AddRelativeLocation` (`self.StaticMesh`) (`KismetMathLibrary.MakeVector` (* _leonmovement_x -1.0 2.0) (* _leonmovement_y 2.0)) false true)
  (if (and (`self.bSnowHasMaxShape`) _returnvalue_2 (not (`/Game/Blueprints/Games/Snowman/BP_SnowmanGame.IsSomeSnowOnAnnaPlace` (`self.SnowmanGame`))) _result)
    (`SceneComponent.K2_SetWorldLocation` (`self.StaticMesh`) _returnvalue false false)
    (set `self.ActorInteractionInfo` (make `/Game/Blueprints/Interaction/S_ObjectInteractionInfo` "NewEnumerator1"))
    (bind _asbpw_interaction_type_widget (cast `/Game/Blueprints/Widgets/Actors/BPW_InteractionTypeWidget` (`WidgetComponent.GetWidget` (`self.Widget`))))
    (bind _asbp_two_characters_controller_2 (cast `/Game/Blueprints/Core/BP_TwoCharactersController` (`GameplayStatics.GetPlayerController` 0)))
    (`/Game/Blueprints/Core/BP_BasePlayer.ShowReaction` (`/Game/Blueprints/Core/BP_TwoCharactersController.Leon` _asbp_two_characters_controller_2) "Поставь снежный ком на место!")
    (`/Game/Blueprints/Widgets/Actors/BPW_InteractionTypeWidget.SetType` _asbpw_interaction_type_widget "NewEnumerator1" "NewEnumerator0")
    (set `self.bSnowReadySet` true)
    (`/Game/Blueprints/Interaction/ActionHandlers/BP_HoldInteractionHandler.SetNewOpt` (`self.BP_HoldInteractionHandler`))
    (elif (and _returnvalue_2 (not _result))
      (bind _asbp_two_characters_controller_3 (cast `/Game/Blueprints/Core/BP_TwoCharactersController` (`GameplayStatics.GetPlayerController` 0)))
      (`/Game/Blueprints/Core/BP_BasePlayer.ShowReaction` (`/Game/Blueprints/Core/BP_TwoCharactersController.Anna` _asbp_two_characters_controller_3) "В основании ставится ком больше!"))))

(event `self.ReceiveTick`
  (params (DeltaSeconds :type "Float (single-precision)"))
  (`parent.ReceiveTick` DeltaSeconds))

(event `/Game/Blueprints/Interaction/BPI_Interactable.HoldInteract`
  (params (InvistigaterCharacter :type "/Game/Blueprints/Core/BP_BasePlayer Object Reference"))
  (`self.CheckCanInteract`)
  (if (`self.bCanInteract`)
    (if (not (`self.bSnowReadySet`))
      (bind _asbp_two_characters_controller (cast `/Game/Blueprints/Core/BP_TwoCharactersController` (`GameplayStatics.GetPlayerController` 0)))
      (bind (_leonmovement_x _leonmovement_y) (`KismetMathLibrary.BreakVector2D` (`/Game/Blueprints/Core/BP_TwoCharactersController.LeonMovement` _asbp_two_characters_controller)))
      (bind _returnvalue (+ (`KismetMathLibrary.Abs` _leonmovement_x) (`KismetMathLibrary.Abs` _leonmovement_y)))
      (if (not (== _returnvalue 0.0))
        (`/Game/Blueprints/Interaction/ActionHandlers/BP_HoldProgressHandler.AddProgress` (`self.BP_HoldProgressHandler`) (/ _returnvalue 30.0))
        (`self.SnowUpdated`))
      (else
        (`/Game/Blueprints/Interaction/ActionHandlers/BP_HoldInteractionHandler.Hold` (`self.BP_HoldInteractionHandler`) InvistigaterCharacter)
        (`self.SnowUpdated`)))))

(fn `GetProgressPercent`
  (returns (Percent :type "Float (double-precision)"))
  (bind _holddestinationseconds (`/Game/Blueprints/Interaction/ActionHandlers/BP_HoldInteractionHandler.HoldDestinationSeconds` (`self.BP_HoldInteractionHandler`)))
  (bind _returnvalue (/ (`KismetMathLibrary.FClamp` (`/Game/Blueprints/Interaction/ActionHandlers/BP_HoldInteractionHandler.CurrentHoldSeconds` (`self.BP_HoldInteractionHandler`)) 0.0 _holddestinationseconds) _holddestinationseconds))
  (`KismetSystemLibrary.PrintString` (`KismetStringLibrary.Conv_DoubleToString` _returnvalue))
  (return _returnvalue))

(fn `UserConstructionScript`
  (`parent.UserConstructionScript`))